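; Showcase actor that automatically sweeps an aim offset through its yaw and pitch range for an animation overview display.
; Tick steps Yaw one unit per frame back and forth across three Pitch rows (up, level, down), feeding variables the mesh's AnimBP reads.
; Chained DoOnce gates initialize each row and reset afterward to loop the sweep.
; The construction script sets the display label from Text.
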(event `ResetDoOnce_1`
  (goto _label :!via `Reset`))

(event `self.ReceiveTick`
  (params (DeltaSeconds :type "Float (single-precision)"))
  (bind _yaw (`self.Yaw`))
  (bind _yaw_2 (`self.Yaw`))
  (bind _yaw_3 (`self.Yaw`))
  (`|ExecutionSequence`
    (:`then_0`
      ;[1 1 1] Update Yaw and Pitch variables based on Slider Blueprints
      (`/Engine/EditorBlueprintResources/StandardMacros.DoOnce` false :!label _label
        (:`Completed`
          (set `self.Pitch` 90.0)
          (set `self.Yaw` -90.0) ; These variables are read by the skeletal mesh's animation Blueprint
        )))
    (:`then_1`
      (if (and (>= _yaw_3 -90.0) (<= _yaw_3 90.0) (== (`self.Pitch`) 90.0))
        (bind _result (`/Engine/EditorBlueprintResources/StandardMacros.IncrementFloat` (`self.Yaw`))
          (:`  `
            (set `self.Yaw` _result) ; These variables are read by the skeletal mesh's animation Blueprint
          ))
        (else
          (`|ExecutionSequence`
            (:`then_0`
              (`/Engine/EditorBlueprintResources/StandardMacros.DoOnce` false :!label _label_2
                (:`Completed`
                  (set `self.Pitch` 0.0)
                  (set `self.Yaw` 89.0) ; These variables are read by the skeletal mesh's animation Blueprint
                )))
            (:`then_1`
              (if (and (>= _yaw -90.0) (<= _yaw 90.0) (== (`self.Pitch`) 0.0))
                (bind _result_2 (`/Engine/EditorBlueprintResources/StandardMacros.DecrementFloat` (`self.Yaw`))
                  (:`  `
                    (set `self.Yaw` _result_2) ; These variables are read by the skeletal mesh's animation Blueprint
                  ))
                (else
                  (`|ExecutionSequence`
                    (:`then_0`
                      (`/Engine/EditorBlueprintResources/StandardMacros.DoOnce` false :!label _label_3
                        (:`Completed`
                          (set `self.Pitch` -90.0)
                          (set `self.Yaw` -89.0) ; These variables are read by the skeletal mesh's animation Blueprint
                        )))
                    (:`then_1`
                      (if (and (>= _yaw_2 -90.0) (<= _yaw_2 90.0) (== (`self.Pitch`) -90.0))
                        (bind _result_3 (`/Engine/EditorBlueprintResources/StandardMacros.IncrementFloat` (`self.Yaw`))
                          (:`  `
                            (set `self.Yaw` _result_3) ; These variables are read by the skeletal mesh's animation Blueprint
                          ))
                        (else
                          (`self.ResetDoOnce_1`)
                          (`self.ResetDoOnce_3`)
                          (`self.ResetDoOnce_2`))))))))))))))

(event `ResetDoOnce_2`
  (goto _label_2 :!via `Reset`))

(event `ResetDoOnce_3`
  (goto _label_3 :!via `Reset`))

(fn `UserConstructionScript`
  (`TextRenderComponent.K2_SetText` (`self.TXT1`) (`self.Text`)))